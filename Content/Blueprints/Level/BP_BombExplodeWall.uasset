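; A destructible wall that reacts to fire-type environment damage, breaking through a Geometry Collection and Chaos fields.
; On the first fire hit only, it spawns a double-scale master field at the collection's location and adds a persistent sleeping-threshold field to it.
; It then deactivates the field system components of the collection's initialization fields.
; Nodes to expire the spawned field and disable the blocking mesh's collision exist but are unconnected.
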(event EventRecieveEnvironmentDamage
  (params (environmentDamageData :type F%20Environment%20Damage%20Structure) (damageSound :type Sound%20Cue%20Object%20Reference))
  (switch Utilities|FlowControl|Switch|SwitchonE_EnvironmentDamage (.damageType (Utilities|Struct|BreakF_EnvironmentDamage environmentDamageData))
    (:NewEnumerator1
      (Utilities|FlowControl|DoOnce false
        (:Completed
          (bind _returnvalue (Game|SpawnActorfromClass "/Game/AlanBreakableWallTest/BP_FS_MasterFieldJim.BP_FS_MasterFieldJim_C" (Math|Transform|MakeTransform (Transformation|GetWorldLocation (Variables|Default|GetGeometryCollection)) "0, 0, 0" "2.000000,2.000000,2.000000") "AlwaysSpawn" "MultiplyWithRoot" 0 0))
          (Class|FieldSystemComponent|AddPersistentField (Variables|/Script/FieldSystemEngine.FieldSystemActor|GetFieldSystemComponent _returnvalue) true "Field_SleepingThreshold")
          (for _array_element (Variables|/Script/GeometryCollectionEngine.GeometryCollectionComponent|GetInitializationFields (Variables|Default|GetGeometryCollection))
            (Components|Activation|SetActive (Variables|/Script/FieldSystemEngine.FieldSystemActor|GetFieldSystemComponent _array_element) false false)))))))

(fn ConstructionScript)