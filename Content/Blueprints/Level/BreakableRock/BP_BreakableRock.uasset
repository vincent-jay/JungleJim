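; Breakable level rock that shatters from player attacks, physics impacts or linked ChainBreak objects, as a standard or explosive variant.
; Standard rocks burst along the hit direction and can drop a coin.
; Explosive rocks boost kicking players; grounded ones damage nearby actors, while floating ones respawn on a timer.
; Pickup rocks attach to a socket, throw with timed downward force, and use timers for interact prompts and a line-traced shadow.
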(event Custom|BreakFromChain
  (params (attackType :type E_Player_AttackTypes%20Enum :default "NewEnumerator6") (attackComponent :type Primitive%20Component%20Object%20Reference) (attackedComponent :type Primitive%20Component%20Object%20Reference))
  (Utilities|IsValid attackComponent
    (:Is%20Valid
      (Utilities|IsValid attackedComponent
        (:Is%20Valid
          (CallFunction|RecievePlayerAttack 0.0 attackType "0, 0, 0" "0, 0, 0" attackComponent attackedComponent))))))

(event Custom|Respawn
  ;[0.1177 0.02692 0.05186] Recieve Player Attack
  (Niagara|SpawnSystematLocation "/Game/Art/Effects/Niagara/Systems/ExplodeRock/NS_ExplodingRock_FloatRegenerate.NS_ExplodingRock_FloatRegenerate" (Transformation|GetWorldLocation (Variables|Default|GetStaticMesh)))
  (Utilities|FlowControl|Delay 0.9)
  (Components|Activation|Activate (Variables|Default|GetFloatingMagicIdle) false)
  (Collision|SetActorEnableCollision true)
  (CallFunction|ReopenAttackGate))

(event Custom|ReopenAttackGate
  ;[0.1177 0.02692 0.05186] Recieve Player Attack
  (Utilities|FlowControl|DoOnce false) ; enters at Reset
)

(event EventBeginPlay
  ;[0.08438 0.02371 0.0704] Setup Shadow
  (if (.canbepickedup (Variables|Default|Getexplodes))
    (Utilities|Time|SetTimerbyFunctionName 0 "ShadowMove" 0.1 true)
    (Variables|Default|SetdisplayShadow true)
    (elif (Variables|Default|Getfloating)
      (CallFunction|ShadowMove)
      (Variables|Default|SetdisplayShadow true)))
  (if (.canbepickedup (Variables|Default|Getexplodes))
    (Utilities|Time|SetTimerbyFunctionName 0 "CheckPlayerDistance" 0.2 true))
  (Utilities|FlowControl|Sequence
    (:then_0
      (Utilities|FlowControl|Delay 1.0)
      (Variables|Default|SethitEventEnabled true))
    (:then_1
      (for _array_element (Variables|Default|GetchainBreak)
        (Utilities|IsValid _array_element
          (:Is%20Valid
            (EventDispatchers|BindEventtoIsBroken _array_element (delegate Custom|BreakFromChain))))))))

(event Collision|EventHit
  (params (MyComp :type Primitive%20Component%20Object%20Reference) (Other :type Actor%20Object%20Reference) (OtherComp :type Primitive%20Component%20Object%20Reference) (bSelfMoved :type Boolean) (HitLocation :type Vector :default "0, 0, 0") (HitNormal :type Vector :default "0, 0, 0") (NormalImpulse :type Vector :default "0, 0, 0") (Hit :type Hit%20Result%20Structure%20%28by%20ref%29))
  (if (Variables|Default|GethitEventEnabled)
    (bind _returnvalue (Physics|GetPhysicsLinearVelocity (Variables|Default|GetStaticMesh) "None"))
    (if (> (Math|Vector|VectorLength _returnvalue) 1.5e+02)
      (CallFunction|RecievePlayerAttack 1.0 "NewEnumerator0" "0, 0, 0" "0, 0, 0"))))

(event EventSetDeactivateUponDeath
  (params (deactivateTrue :type Boolean))
  (Variables|TimerChallenge|SetdeactivateUponDeath deactivateTrue))

(event EventResetIsDeactivatedVar
  (Variables|TimerChallenge|Setdeactivated false))

(event EventRecievePlayerAttack
  (params (attackDamage :type Float%20%28double-precision%29) (attackType :type E_Player_AttackTypes%20Enum :default "NewEnumerator6") (attackVelocity :type Vector :default "0, 0, 0") (attackLocation :type Vector :default "0, 0, 0") (attackComponent :type Primitive%20Component%20Object%20Reference) (attackedComponent :type Primitive%20Component%20Object%20Reference))
  ;[0.1177 0.02692 0.05186] Recieve Player Attack
  (Utilities|FlowControl|DoOnce false
    (:Completed
      (Default|CallIsBroken attackType attackComponent attackedComponent)
      (EventDispatchers|UnbindallEventsfromIsBroken)
      (Rendering|SetVisibility (Variables|Default|GetStaticMesh) false false)
      (Collision|SetActorEnableCollision false)
      (if (.canexplode (Variables|Default|Getexplodes))
        (|MagicExplosionRock attackType)
        (else
          (|StandardRock attackType attackComponent attackedComponent))))))

(event EventTick
  (params (DeltaSeconds :type Float%20%28single-precision%29))
  (bind _indicator_pivot (Variables|Default|GetIndicator_Pivot)
    (:then
      (Transformation|SetWorldLocation _indicator_pivot (+ (Transformation|GetWorldLocation (Variables|Default|GetStaticMesh)) "0.000000,0.000000,60.000000") false false))
    (:else)))

(fn ConstructionScript
  (bind _explodes (Variables|Default|Getexplodes))
  (Effects|Components|ParticleSystem|SetVectorParameter (Variables|Default|GetDestroyVFX) "scale" (Transformation|GetActorScale3D))
  (Effects|Components|ParticleSystem|SetFloatParameter (Variables|Default|GetDestroyVFX) "scaleFloat" (.z (Transformation|GetActorScale3D)))
  (if (.canexplode _explodes)
    (Rendering|Material|SetMaterial (Variables|Default|GetStaticMesh) 0 "/Game/Art/Environment/Rocky/BreakableRock/MI_BreakableRock_ExplodePlaceholder.MI_BreakableRock_ExplodePlaceholder")
    (if (Variables|Default|Getfloating)
      (Collision|SetCollisionEnabled (Variables|Default|GetStaticMesh) "NoCollision")
      (Rendering|SetVisibility (Variables|Default|GetStaticMesh) false false)
      (Rendering|SetVisibility (Variables|Default|GetShadowDecal) true false)
      (Components|Activation|SetAutoActivate (Variables|Default|GetFloatingMagicIdle) true)
      (else
        (Components|Activation|SetAutoActivate (Variables|Default|GetFloatingMagicIdle) false :!label _label)
        (if (.canbepickedup _explodes) ; Interactable / Throwable object
          (Physics|SetSimulatePhysics (Variables|Default|GetStaticMesh) true))))
    (else
      (goto _label))))

(fn GetFlipKickLaunch
  (bind _returnvalue (Game|Player|GetPlayerPawn 0))
  (return (* (Math|Vector|Lerp(Vector) (Transformation|GetActorForwardVector _returnvalue) (Transformation|GetActorUpVector _returnvalue) (Variables|Default|LaunchAngles|GetflipKickLaunchAlpha)) (.launchstrength (Variables|Default|Getexplodes)))))

(fn GetDiveKickLaunch
  (bind _returnvalue (Game|Player|GetPlayerPawn 0))
  (return (* (Math|Vector|Lerp(Vector) (Transformation|GetActorForwardVector _returnvalue) (Transformation|GetActorUpVector _returnvalue) (Variables|Default|LaunchAngles|GetdiveKickLaunchAlpha)) (.launchstrength (Variables|Default|Getexplodes)))))

(fn AttachtoOwner
  (params (OwningActor :type BP%20Player%20Base%20Object%20Reference) (attachName :type Name))
  (bind _staticmesh (Variables|Default|GetStaticMesh))
  (Variables|Default|Interaction|SetOwningActor OwningActor)
  (Physics|SetSimulatePhysics _staticmesh false)
  (Collision|SetCollisionEnabled _staticmesh "PhysicsOnly")
  (Transformation|AttachComponentToComponent (Variables|/Script/Engine.Character|GetMesh (Variables|Default|Interaction|GetOwningActor)) attachName "SnapToTarget" "SnapToTarget" "KeepWorld" true))

(fn DetachfromOwner
  (bind _staticmesh (Variables|Default|GetStaticMesh))
  (bind _holdsocket (Variables|Default|Interaction|GetholdSocket))
  (bind _owningactor (Variables|Default|Interaction|GetOwningActor))
  (bind _mesh (Variables|/Script/Engine.Character|GetMesh _owningactor))
  (bind _returnvalue (Transformation|GetSocketTransform _mesh _holdsocket "RTS_World"))
  (Transformation|DetachFromActor self "KeepWorld" "KeepRelative" "KeepWorld")
  (Transformation|SetActorLocationAndRotation (.location _returnvalue) (.rotation _returnvalue))
  (Physics|SetSimulatePhysics _staticmesh true)
  (Collision|SetCollisionResponsetoChannel _staticmesh "ECC_Pawn" "ECR_Ignore")
  (Collision|SetCollisionEnabled _staticmesh "QueryAndPhysics"))

(fn ResetPawnResponseChannel
  (Collision|SetCollisionResponsetoChannel (Variables|Default|GetStaticMesh) "ECC_Pawn" "ECR_Block"))

(fn CanThisbeInteracted
  (return (.canbepickedup (Variables|Default|Getexplodes))))

(event Custom|SystemFinished
  (params (PSystem :type Niagara%20Component%20Object%20Reference))
  (if (Variables|TimerChallenge|GetdeactivateUponDeath)
    ;[0.1135 0.1135 0.1135] Deactivate Actor
    (Collision|SetActorEnableCollision false)
    (Rendering|SetActorHiddenInGame true)
    (Variables|TimerChallenge|Setdeactivated true)
    ;[0.06354 0.06354 0.06354] Reset State
    (Rendering|SetVisibility (Variables|Default|GetStaticMesh) true false)
    (CallFunction|ReopenAttackGate)
    (else
      (Actor|DestroyActor))))

(event Custom|PickUp
  (params (InteractPlayer :type BP%20Player%20Base%20Object%20Reference))
  ;[0.176 0.176 0.176] Pickup
  (if (Variables|Default|Interaction|GetcanBeInteracted)
    (CallFunction|AttachtoOwner InteractPlayer (Variables|Default|Interaction|GetholdSocket))
    (Variables|Default|Interaction|SetcanBeInteracted false)
    (Components|Activation|Deactivate (Variables|Default|GetNS_InteractIndicator))))

(event Custom|Drop
  ;[0.1385 0.1385 0.1385] Drop
  (CallFunction|DetachfromOwner)
  (Variables|Default|Interaction|SetOwningActor 0)
  (Utilities|Time|SetTimerbyFunctionName 0 "Reset Pawn Response Channel" 0.2)
  (CallFunction|ApplyDownwardForce)
  (Variables|Default|Interaction|SetcanBeInteracted true)
  (Variables|Default|SethitEventEnabled false)
  (Utilities|FlowControl|Delay 0.5)
  (Variables|Default|SethitEventEnabled true))

(event Custom|ApplyThrowLaunchForce
  ;[0.1344 0.1344 0.1344] Throw
  (Physics|AddForce (Variables|Default|GetStaticMesh) (* (Math|Vector|VectorUp) -2.8e+06) "None" false))

(event Custom|Throw
  (bind _staticmesh (Variables|Default|GetStaticMesh))
  ;[0.1344 0.1344 0.1344] Throw
  (Variables|Default|Interaction|SetcanBeInteracted true)
  (CallFunction|DetachfromOwner)
  (bind _returnvalue (Physics|GetPhysicsLinearVelocity _staticmesh "None"))
  (Class|PrimitiveComponent|SetAllPhysicsLinearVelocity _staticmesh (Math|Vector|MakeVector (/ (.x _returnvalue) 3.0) (/ (.y _returnvalue) 3.0) 0.0) false)
  (Physics|AddImpulse (Variables|Default|GetStaticMesh) (* (+ (Transformation|GetActorForwardVector (Variables|Default|Interaction|GetOwningActor)) (* (Transformation|GetActorUpVector (Variables|Default|Interaction|GetOwningActor)) 0.8)) 9e+05) "None" false)
  (Variables|Default|Interaction|SetOwningActor 0)
  (Utilities|Time|SetTimerbyFunctionName 0 "Reset Pawn Response Channel" 0.2)
  (bind _returnvalue_2 (Utilities|Time|SetTimerbyEvent (delegate Custom|ApplyThrowLaunchForce) 0.05 true))
  (Utilities|FlowControl|Delay 0.75)
  (Utilities|Time|ClearandInvalidateTimerbyHandle _returnvalue_2))

(event Custom|CheckPlayerDistance
  (bind _interactarrow (Variables|Default|GetInteractArrow))
  (bind _interactarrow_2 (Variables|Default|GetInteractArrow))
  ;[0.1594 0.1594 0.1594 1 32] Interact VFX
  (Utilities|IsValid (Game|Player|GetPlayerPawn 0)
    (:Is%20Valid
      (if (Variables|Default|Interaction|GetcanBeInteracted)
        (Class|NiagaraComponent|SetVariableMaterial (Variables|Default|GetNS_InteractIndicator) "interactIcon" (Utilities|Select :Index (Class|CommonInputSubsystem|GetCurrentInputType (PlayerController|LocalPlayerSubsystems|GetCommonInputSubsystem (Game|GetPlayerController 0))) :MouseAndKeyboard "/Game/Art/UI/InputUI/M_UI_Interact_Keyboard.M_UI_Interact_Keyboard" :Gamepad "/Game/Art/UI/InputUI/MI_UI_Interact_Gamepad.MI_UI_Interact_Gamepad" :Touch "/Game/Art/UI/InputUI/MI_UI_Interact_Gamepad.MI_UI_Interact_Gamepad" :Count "/Game/Art/UI/InputUI/MI_UI_Interact_Gamepad.MI_UI_Interact_Gamepad"))
        (Components|Activation|Deactivate (Variables|Default|GetInteractArrow))
        (Components|Activation|Activate (Variables|Default|GetNS_InteractIndicator) false)
        (else
          (Components|Activation|Deactivate (Variables|Default|GetNS_InteractIndicator))))
      (Variables|Default|Interaction|GetOwningActor
        (:then
          (if (and (Components|Activation|IsActive (Variables|Default|GetInteractArrow)) (not (Audio|Components|Audio|IsPlaying (Variables|Default|GetArrowDisappear)))) :!label _label
            (Components|Timeline|SetPlayRate (Variables|Default|GetArrowDisappear) 3.0)
            (bind (_direction _arrowscale _arrowposition) (Timeline|ArrowDisappear PlayFromStart)
              (:Update
                (Class|NiagaraComponent|SetVariableVec2 _interactarrow_2 "ArrowScale" (Math|Conversions|ToVector2D(Vector) _arrowscale))
                (Niagara|SetNiagaraVariable(Vector3) _interactarrow_2 "ArrowPosition" _arrowposition))
              (:Finished
                (Components|Activation|Deactivate (Variables|Default|GetInteractArrow))))))
        (:else
          (if (<= (Math|Vector|Distance(Vector) (Transformation|GetActorLocation (Game|Player|GetPlayerPawn 0)) (Transformation|GetActorLocation)) (Variables|Default|Interaction|GetinteractArrowDistance))
            (if (not (or (Components|Activation|IsActive (Variables|Default|GetInteractArrow)) (Variables|Default|Interaction|GetcanBeInteracted)))
              (Components|Activation|Activate (Variables|Default|GetInteractArrow) false)
              (Components|Timeline|SetPlayRate (Variables|Default|GetArrowAppear) 2.0)
              (bind (_direction_2 _arrowscale_2 _arrowposition_2) (Timeline|ArrowAppear PlayFromStart)
                (:Update
                  (Class|NiagaraComponent|SetVariableVec2 _interactarrow "ArrowScale" (Math|Conversions|ToVector2D(Vector) _arrowscale_2))
                  (Niagara|SetNiagaraVariable(Vector3) _interactarrow "ArrowPosition" _arrowposition_2))))
            (else
              (goto _label))))))))

(event Custom|ApplyDownwardForce
  ;[0.1344 0.1344 0.1344] Throw
  (bind _returnvalue (Utilities|Time|SetTimerbyEvent (delegate Custom|ApplyThrowLaunchForce) 0.05 true))
  (Utilities|FlowControl|Delay 0.75)
  (Utilities|Time|ClearandInvalidateTimerbyHandle _returnvalue))

(event EventInteractCanbeInteracted
  (params (canBeInteracted :type Boolean))
  ;[0.1594 0.1594 0.1594 1 32] Interact VFX
  (Variables|Default|Interaction|SetcanBeInteracted canBeInteracted))

(event EventSetCollision
  (params (newCollision :type ECollisionEnabled%20Enum :default "NoCollision"))
  ;[0.1594 0.1594 0.1594 1 32] Interact VFX
  (Collision|SetCollisionEnabled (Variables|Default|GetStaticMesh) newCollision))

(event EventInteract
  (params (interactState :type E_InteractState%20Enum :default "NewEnumerator4") (InteractPlayer :type BP%20Player%20Base%20Object%20Reference))
  ;[0.1344 0.1344 0.1344 1 30] Interact Event
  (switch Utilities|FlowControl|Switch|SwitchonE_InteractState interactState
    (:NewEnumerator0
      (CallFunction|PickUp InteractPlayer))
    (:NewEnumerator1
      (CallFunction|Throw))
    (:NewEnumerator2
      (CallFunction|Drop))))

(event Custom|ShadowMove
  (bind _self self)
  (bind _staticmesh (Variables|Default|GetStaticMesh))
  (bind _staticmesh_2 (Variables|Default|GetStaticMesh))
  (bind _returnvalue (Transformation|GetWorldLocation _staticmesh_2))
  (bind _returnvalue_2 (Transformation|GetWorldLocation _staticmesh))
  (bind _returnvalue_3 (Transformation|GetActorLocation _self))
  (bind _returnvalue_4 (Math|Vector|Lerp(Vector) _returnvalue_2 _returnvalue_3 0.5))
  ;[0.1009 0.0473 0.1094] Shadow Move
  (bind (_outhit _returnvalue_5) (Collision|LineTraceByChannel _returnvalue_4 (+ _returnvalue_4 (* (Transformation|GetActorUpVector _self) -4e+03)) "TraceTypeQuery1" false 0 "None" true "(R=1.000000,G=0.000000,B=0.000000,A=1.000000)" "(R=0.000000,G=1.000000,B=0.000000,A=1.000000)" 1.0))
  (if _returnvalue_5
    (if (Actor|ActorHasTag (.HitActor (Collision|BreakHitResult _outhit)) "Water")
      (Rendering|SetVisibility (Variables|Default|GetBackupShadow) true false)
      (Transformation|SetWorldLocationAndRotation (Variables|Default|GetBackupShadow) (Math|Vector|MakeVector (.X (Math|Vector|BreakVector (.ImpactPoint (Collision|BreakHitResult _outhit)))) (.Y (Math|Vector|BreakVector (.ImpactPoint (Collision|BreakHitResult _outhit)))) (+ (.Z (Math|Vector|BreakVector (.ImpactPoint (Collision|BreakHitResult _outhit)))) 4.0)) (Math|Rotator|MakeRotfromZ (.ImpactNormal (Collision|BreakHitResult _outhit))) false false)
      (else
        (Rendering|SetVisibility (Variables|Default|GetBackupShadow) false false)
        (Transformation|SetWorldLocation (Variables|Default|GetShadowDecal) (Math|Vector|MakeVector (.x _returnvalue) (.y _returnvalue) (.z (.Location (Collision|BreakHitResult _outhit)))) false false)
        (if (<= (.Distance (Collision|BreakHitResult _outhit)) 1.5e+03)
          (Transformation|SetWorldScale3D (Variables|Default|GetShadowDecal) (Math|Vector|MakeVector 1.0 (Math|Float|Lerp 1.3 0.4 (Math|Float|Clamp(Float) (/ (.Distance (Collision|BreakHitResult _outhit)) 1.25e+03))) (Math|Float|Lerp 1.3 0.4 (Math|Float|Clamp(Float) (/ (.Distance (Collision|BreakHitResult _outhit)) 1.25e+03)))))
          (else
            (Transformation|SetWorldScale3D (Variables|Default|GetShadowDecal) (Math|Vector|MakeVector 0.0 0.0 0.0))))))
    (else
      (Rendering|SetVisibility (Variables|Default|GetBackupShadow) false false))))

(event Custom|DestroyRock
  (params (PSystem :type Niagara%20Component%20Object%20Reference))
  (if (Variables|TimerChallenge|GetdeactivateUponDeath)
    ;[0.1135 0.1135 0.1135] Deactivate Actor
    (Collision|SetActorEnableCollision false)
    (Rendering|SetActorHiddenInGame true)
    (Variables|TimerChallenge|Setdeactivated true)
    ;[0.06354 0.06354 0.06354] Reset State
    (Rendering|SetVisibility (Variables|Default|GetStaticMesh) true false)
    (CallFunction|ReopenAttackGate)
    (else
      (Actor|DestroyActor))))

(fn GetDamagedSound
  (return 0))

(fn GetHurtbox
  (return 0))

(fn GetZInteractRangeAddition
  (return 0.0))

(fn IsDeactivated
  (return (Variables|TimerChallenge|Getdeactivated)))

(fn ShouldFlash
  (return (Variables|TimerChallenge|GetshouldFlashInTimerChallenge)))