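; Music manager for the Rhythmic Ruins level that keeps gameplay events in time with the soundtrack through Quartz.
; On BeginPlay it creates a 4/4 Quartz clock at the configured BPM, starts the music quantized to the beat, and caches all BP_BeatPlatform actors.
; A quarter-note subscription prints the bar and beat for debugging and calls OnBeat with both values.
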(event Custom|Start%20Clock
  (bind _clockhandle (Class|QuartzClockHandle|StartClock (Variables|Default|GetClock%20Handle)))
  (Audio|Components|Audio|PlayQuantized (Variables|Default|GetMusicComponent) _clockhandle (Utilities|Struct|MakeQuartzQuantizationBoundary "Beat" 1.0 "BarRelative" true false false false) 0)
  (Class|QuartzClockHandle|SubscribetoQuantizationEvent (Variables|Default|GetClock%20Handle) "QuarterNote" (delegate Custom|OnQuarterBeat)))

(event Custom|OnQuarterBeat
  (params (ClockName :type Name) (QuantizationType :type EQuartzCommandQuantization%20Enum :default "Bar") (NumBars :type Integer) (Beat :type Integer) (BeatFraction :type Float%20%28single-precision%29))
  (Development|PrintText (Utilities|Text|FormatText "{bar} / {beat}" NumBars Beat))
  (Default|CallOnBeat Beat NumBars))

(event EventBeginPlay
  (bind _returnvalue (Class|QuartzSubsystem|CreateNewClock (WorldSubsystems|GetQuartzSubsystem) (Variables|Default|GetClock%20Name) (Utilities|Struct|MakeQuartzClockSettings (Utilities|Struct|MakeQuartzTimeSignature 4 "QuarterNote") false) false))
  (bind _output_get (Variables|Default|SetClock%20Handle _returnvalue))
  (Class|QuartzClockHandle|SetBeatsPerMinute :self _output_get :BeatsPerMinute (Variables|Default|GetBPM))
  (CallFunction|StartClock)
  (bind _outactors (Actor|GetAllActorsOfClass "/Game/Levels/RhythmicRuins/Blueprints/BP_BeatPlatform.BP_BeatPlatform_C"))
  (Variables|Default|SetOn%20Beat%20Actors _outactors))

(fn ConstructionScript)