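; BP_BeatPlatform is a Rhythmic Ruins platform that slides in and out to the music's beat.
; It binds to the OnBeat event of BP_RRMusicManager and looks up the current beat in a bool pattern to decide whether to be out or in.
; A timeline moves the platform along a spline, playing forward to extend and reversing to retract.
; Collision turns on as extension starts and off as retraction starts.
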(event Custom|Push%20Platform%20Out
  (if (not (Variables|Default|GetPlatformOut))
    (Variables|Default|SetPlatformOut true)
    (Collision|SetCollisionEnabled (Variables|Default|GetPlatform) "QueryAndPhysics")
    (bind _track (Timeline|Push%20Platform PlayFromStart)
      (:Update
        (Transformation|SetWorldLocation (Variables|Default|GetPlatform) (Spline|GetLocationatDistanceAlongSpline (Variables|Default|GetSpline) (Math|Float|Lerp 0.0 4e+02 _track) "World") false false)))))

(event Custom|Pull%20Platform%20In
  (if (Variables|Default|GetPlatformOut)
    (Variables|Default|SetPlatformOut false)
    (Collision|SetCollisionEnabled (Variables|Default|GetPlatform) "NoCollision")
    (bind _track (Timeline|Push%20Platform ReverseFromEnd)
      (:Update
        (Transformation|SetWorldLocation (Variables|Default|GetPlatform) (Spline|GetLocationatDistanceAlongSpline (Variables|Default|GetSpline) (Math|Float|Lerp 0.0 4e+02 _track) "World") false false)))))

(event Custom|On%20Beat
  (params (Beat :type Integer) (Num%20Bars :type Integer))
  (if (Utilities|Array|Get(acopy) (Variables|Default|GetOutBeats) (- Beat 1))
    (CallFunction|PushPlatformOut)
    (else
      (CallFunction|PullPlatformin))))

(event EventBeginPlay
  (bind _returnvalue (Actor|GetActorOfClass "/Game/Levels/RhythmicRuins/Blueprints/BP_RRMusicManager.BP_RRMusicManager_C"))
  (EventDispatchers|BindEventtoOnBeat _returnvalue (delegate Custom|On%20Beat)))

(fn ConstructionScript)