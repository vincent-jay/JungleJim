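; Breakable barrel that shatters on the first player attack it receives and can drop an item.
; Each handled melee attack type leads to the same break, spawning a short-lived BP_FS_MasterFieldJim field system at the hit location with a persistent sleeping-threshold field.
; It then disables BlockingMesh collision and spawns the optional ItemDrop class at the barrel's location.
; GetDamagedSound and GetHurtbox are empty stubs.
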(event EventRecievePlayerAttack
  (params (attackDamage :type Float%20%28double-precision%29) (attackType :type E_Player_AttackTypes%20Enum :default "NewEnumerator6") (attackVelocity :type Vector :default "0, 0, 0") (attackLocation :type Vector :default "0, 0, 0") (attackComponent :type Primitive%20Component%20Object%20Reference) (attackedComponent :type Primitive%20Component%20Object%20Reference))
  (Utilities|FlowControl|DoOnce false
    (:Completed
      (switch Utilities|FlowControl|Switch|SwitchonE_Player_AttackTypes attackType
        (:NewEnumerator5
          _)
        (:NewEnumerator0
          _)
        (:NewEnumerator4
          _)
        (:NewEnumerator1
          _)
        (:NewEnumerator7
          _)
        (:NewEnumerator8
          _)
        (:NewEnumerator2
          _)
        (:NewEnumerator10
          _)
        (:NewEnumerator11
          _))
      (bind _returnvalue (Game|SpawnActorfromClass "/Game/AlanBreakableWallTest/BP_FS_MasterFieldJim.BP_FS_MasterFieldJim_C" (Math|Transform|MakeTransform attackLocation "0, 0, 0" "2.000000,2.000000,2.000000") "AlwaysSpawn" "MultiplyWithRoot" 0 0))
      (Class|FieldSystemComponent|AddPersistentField (Variables|/Script/FieldSystemEngine.FieldSystemActor|GetFieldSystemComponent _returnvalue) true "Field_SleepingThreshold")
      (Actor|SetLifeSpan _returnvalue 2.0)
      (Collision|SetCollisionEnabled (Variables|Default|GetBlockingMesh) "NoCollision")
      (bind _itemdrop (Variables|Default|GetitemDrop)
        (:then
          (Game|SpawnActorfromClass _itemdrop (Math|Transform|MakeTransform (Transformation|GetActorLocation)) "AlwaysSpawn" "MultiplyWithRoot" 0 0))
        (:else)))))

(fn ConstructionScript)

(fn GetDamagedSound
  (return 0))

(fn GetHurtbox
  (return 0))